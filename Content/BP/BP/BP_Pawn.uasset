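; BP_Pawn is a pawn that uses gaze from its cine camera to trigger a switch to the SubMain level.
; Every tick, GazeCheck runs a debug-drawn line trace along the camera's forward vector on the Camera channel.
; Hitting a Dummy actor starts a delay of a few seconds before the level opens, with no check that the gaze is held.
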(event `self.ReceiveTick`
  (params (DeltaSeconds :type "Float (single-precision)"))
  (`self.GazeCheck`))

(event `GazeCheck`
  (bind _cinecamera (`self.CineCamera`))
  (bind _returnvalue (`SceneComponent.K2_GetComponentLocation` _cinecamera))
  ;[1 1 1] GazeCheck
  (bind _outhit (`KismetSystemLibrary.LineTraceSingle` :`Start` _returnvalue :`End` (+ _returnvalue (* (`SceneComponent.GetForwardVector` _cinecamera) 1000.0)) :`TraceChannel` "TraceTypeQuery2" :`DrawDebugType` "ForDuration" :`DrawTime` 3.0))
  (cast `/Game/BP/Dummy` (`.HitActor` (`GameplayStatics.BreakHitResult` _outhit)))
  (`KismetSystemLibrary.Delay` 5.0)
  (`GameplayStatics.OpenLevel` "SubMain"))

(fn `UserConstructionScript`)